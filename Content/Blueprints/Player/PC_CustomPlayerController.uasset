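; Custom player controller that toggles the pause screen when the IA_Pause input action fires.
; Pausing creates UMG_MainMenu, shows the cursor, switches to Game and UI input, pauses the game and hides the AstronautCharacter HUD.
; A valid PauseUIRef marks the paused state, so the next press removes the widget and restores game-only input, hidden cursor, gameplay and HUD.
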(event Input|EnhancedActionEvents|EnhancedInputActionIA_Pause
  (params (ActionValue :type Boolean) (ElapsedSeconds :type Float%20%28double-precision%29) (TriggeredSeconds :type Float%20%28double-precision%29) (InputAction :type Input%20Action%20Object%20Reference :default "/Game/Controls/IA_Pause.IA_Pause"))
  (bind _returnvalue (Game|GetPlayerController 0))
  (bind _returnvalue_2 (Game|GetPlayerController 0))
  ;[1 1 1] Control Pause Screen
  (:Triggered
    (Utilities|IsValid (Variables|Default|GetPauseUIRef)
      (:Is%20Valid
        ;[1 1 1] Unpause
        (Widget|RemovefromParent (Variables|Default|GetPauseUIRef))
        (Variables|Default|SetPauseUIRef 0)
        (Input|SetInputModeGameOnly _returnvalue false)
        (Variables|/Script/Engine.PlayerController|SetbShowMouseCursor _returnvalue false)
        (Game|SetGamePaused false)
        (bind _asastronaut_character (Utilities|Casting|CastToAstronautCharacter (Game|Player|GetPlayerPawn 0)))
        (Default|ToggleHUDon _asastronaut_character))
      (:Is%20Not%20Valid
        ;[1 1 1] Pause
        (bind _returnvalue_3 (UserInterface|CreateWidget "/Game/UI/UMG_MainMenu.UMG_MainMenu_C"))
        (bind _output_get (Variables|Default|SetPauseUIRef _returnvalue_3))
        (UserInterface|Viewport|AddtoViewport _output_get 0)
        (Input|SetInputModeGameandUI _returnvalue_2 0 "DoNotLock" true false)
        (Variables|/Script/Engine.PlayerController|SetbShowMouseCursor _returnvalue_2 true)
        (Game|SetGamePaused true)
        (bind _asastronaut_character_2 (Utilities|Casting|CastToAstronautCharacter (Game|Player|GetPlayerPawn 0)))
        (Default|ToggleHUDOff _asastronaut_character_2)))))

(fn ConstructionScript)