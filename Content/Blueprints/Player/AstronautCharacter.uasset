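; Player astronaut character with physics-driven movement and free pitch, yaw and roll rotation.
; Enhanced Input events add to the model's linear velocity or rotate the actor locally, while stabilize lerps linear and angular velocity toward zero.
; Movement and look inputs trigger a camera line trace that updates the HUD's interactable hover state.
; Interact sphere-traces from the camera after a short delay and messages actors implementing BPI_Interaction.
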(event Custom|UpdatedInput
  (bind _hudwidget (Variables|Default|GetHUDWidget))
  (bind _camera (Variables|Camera|GetCamera))
  (bind _returnvalue (Transformation|GetWorldLocation _camera))
  ;[1 1 1] Check for possible interaction
  (bind _outhit (Collision|LineTraceByChannel _returnvalue (+ _returnvalue (* (Math|Vector|GetForwardVector _camera) "400.000000,400.000000,400.000000")) "TraceTypeQuery1" false 0 "None" true "(R=1.000000,G=0.000000,B=0.000000,A=1.000000)" "(R=0.000000,G=1.000000,B=0.000000,A=1.000000)" 1.0))
  (if (.bBlockingHit (Collision|BreakHitResult _outhit))
    (if (Utilities|DoesObjectImplementInterface (.HitActor (Collision|BreakHitResult _outhit)) "/Game/Blueprints/InteractableObjects/BPI_Interaction.BPI_Interaction_C")
      (Default|HoveringOverInteractable _hudwidget true)
      (else
        (Default|HoveringOverInteractable _hudwidget false :!label _label)))
    (else
      (goto _label))))

(event Input|EnhancedActionEvents|EnhancedInputActionIA_Stabilize
  (params (ActionValue :type Boolean) (ElapsedSeconds :type Float%20%28double-precision%29) (TriggeredSeconds :type Float%20%28double-precision%29) (InputAction :type Input%20Action%20Object%20Reference :default "/Game/Controls/IA_Stabilize.IA_Stabilize"))
  (bind _modelasparent (Variables|Default|GetModelAsParent))
  (bind _modelasparent_2 (Variables|Default|GetModelAsParent))
  ;[1 1 1] Stabilization of the character
  (bind _returnvalue (Physics|GetPhysicsLinearVelocity _modelasparent "None"))
  (Physics|SetPhysicsLinearVelocity _modelasparent_2 (Math|Vector|Lerp(Vector) _returnvalue "0, 0, 0" 0.01) false "None")
  (Class|PrimitiveComponent|SetPhysicsAngularVelocityinDegrees _modelasparent_2 (Math|Vector|Lerp(Vector) (Physics|GetPhysicsAngularVelocityinDegrees _modelasparent "None") "0, 0, 0" 0.01) false "None"))

(event Input|EnhancedActionEvents|EnhancedInputActionIA_MouseInputX
  (params (ActionValue :type Float%20%28double-precision%29) (ElapsedSeconds :type Float%20%28double-precision%29) (TriggeredSeconds :type Float%20%28double-precision%29) (InputAction :type Input%20Action%20Object%20Reference :default "/Game/Controls/IA_MouseInputX.IA_MouseInputX"))
  ;[1 1 1] 360 degree freedom movement rotation
  (Transformation|AddActorLocalRotation (Math|Rotator|MakeRotator 0.0 0.0 ActionValue) false false)
  ;[1 1 1] Update LineTrace for UI
  (CallFunction|UpdatedInput))

(event Input|EnhancedActionEvents|EnhancedInputActionIA_ForwardMove
  (params (ActionValue :type Float%20%28double-precision%29) (ElapsedSeconds :type Float%20%28double-precision%29) (TriggeredSeconds :type Float%20%28double-precision%29) (InputAction :type Input%20Action%20Object%20Reference :default "/Game/Controls/IA_ForwardMove.IA_ForwardMove"))
  (bind _modelasparent (Variables|Default|GetModelAsParent))
  ;[1 1 1] Physics Based Movement
  (bind _returnvalue (Physics|GetPhysicsLinearVelocity _modelasparent "None"))
  (Physics|SetPhysicsLinearVelocity _modelasparent (+ _returnvalue (* ActionValue (Transformation|GetActorForwardVector)) (* (stale Input|EnhancedActionEvents|EnhancedInputActionIA_SideMove ActionValue) (Transformation|GetActorRightVector))) false "None")
  ;[1 1 1] Update LineTrace for UI
  (CallFunction|UpdatedInput))

(event Input|EnhancedActionEvents|EnhancedInputActionIA_SideMove
  (params (ActionValue :type Float%20%28double-precision%29) (ElapsedSeconds :type Float%20%28double-precision%29) (TriggeredSeconds :type Float%20%28double-precision%29) (InputAction :type Input%20Action%20Object%20Reference :default "/Game/Controls/IA_SideMove.IA_SideMove"))
  (bind _modelasparent (Variables|Default|GetModelAsParent))
  ;[1 1 1] Physics Based Movement
  (bind _returnvalue (Physics|GetPhysicsLinearVelocity _modelasparent "None"))
  (Physics|SetPhysicsLinearVelocity _modelasparent (+ _returnvalue (* (stale Input|EnhancedActionEvents|EnhancedInputActionIA_ForwardMove ActionValue) (Transformation|GetActorForwardVector)) (* ActionValue (Transformation|GetActorRightVector))) false "None")
  ;[1 1 1] Update LineTrace for UI
  (CallFunction|UpdatedInput))

(event Input|EnhancedActionEvents|EnhancedInputActionIA_MouseInputX
  (params (ActionValue :type Float%20%28double-precision%29) (ElapsedSeconds :type Float%20%28double-precision%29) (TriggeredSeconds :type Float%20%28double-precision%29) (InputAction :type Input%20Action%20Object%20Reference :default "/Game/Controls/IA_MouseInputX.IA_MouseInputX"))
  ;[1 0.8469 0.2831] View and Roll Inputs (Deprecated)
)

(event Input|EnhancedActionEvents|EnhancedInputActionIA_MouseInputY
  (params (ActionValue :type Float%20%28double-precision%29) (ElapsedSeconds :type Float%20%28double-precision%29) (TriggeredSeconds :type Float%20%28double-precision%29) (InputAction :type Input%20Action%20Object%20Reference :default "/Game/Controls/IA_MouseInputY.IA_MouseInputY"))
  ;[1 0.8469 0.2831] View and Roll Inputs (Deprecated)
)

(event Input|EnhancedActionEvents|EnhancedInputActionIA_Interact
  (params (ActionValue :type Boolean) (ElapsedSeconds :type Float%20%28double-precision%29) (TriggeredSeconds :type Float%20%28double-precision%29) (InputAction :type Input%20Action%20Object%20Reference :default "/Game/Controls/IA_Interact.IA_Interact"))
  (bind _camera (Variables|Camera|GetCamera))
  (bind _returnvalue (Transformation|GetWorldLocation _camera))
  ;[1 1 1] Interact Event Interaction BPI
  (Utilities|FlowControl|Delay 0.1)
  (bind _outhit (Collision|SphereTraceByChannel _returnvalue (+ _returnvalue (* (Math|Vector|GetForwardVector _camera) "400.000000,400.000000,400.000000")) 3.0 "TraceTypeQuery1" false 0 "ForDuration"))
  (if (.bBlockingHit (Collision|BreakHitResult _outhit))
    (if (Utilities|DoesObjectImplementInterface (.HitActor (Collision|BreakHitResult _outhit)) "/Game/Blueprints/InteractableObjects/BPI_Interaction.BPI_Interaction_C")
      (Class|BPIInteraction|Interact(Message) (.HitActor (Collision|BreakHitResult _outhit))))))

(event Input|EnhancedActionEvents|EnhancedInputActionIA_ForwardMove
  (params (ActionValue :type Float%20%28double-precision%29) (ElapsedSeconds :type Float%20%28double-precision%29) (TriggeredSeconds :type Float%20%28double-precision%29) (InputAction :type Input%20Action%20Object%20Reference :default "/Game/Controls/IA_ForwardMove.IA_ForwardMove"))
  ;[1 0.8469 0.2831] Movement Forward and Sideways (Deprecated)
)

(event Input|EnhancedActionEvents|EnhancedInputActionIA_SideMove
  (params (ActionValue :type Float%20%28double-precision%29) (ElapsedSeconds :type Float%20%28double-precision%29) (TriggeredSeconds :type Float%20%28double-precision%29) (InputAction :type Input%20Action%20Object%20Reference :default "/Game/Controls/IA_SideMove.IA_SideMove"))
  ;[1 0.8469 0.2831] Movement Forward and Sideways (Deprecated)
)

(event Input|EnhancedActionEvents|EnhancedInputActionIA_Roll
  (params (ActionValue :type Float%20%28double-precision%29) (ElapsedSeconds :type Float%20%28double-precision%29) (TriggeredSeconds :type Float%20%28double-precision%29) (InputAction :type Input%20Action%20Object%20Reference :default "/Game/Controls/IA_Roll.IA_Roll"))
  ;[1 0.8469 0.2831] View and Roll Inputs (Deprecated)
)

(event Input|EnhancedActionEvents|EnhancedInputActionIA_MouseInputY
  (params (ActionValue :type Float%20%28double-precision%29) (ElapsedSeconds :type Float%20%28double-precision%29) (TriggeredSeconds :type Float%20%28double-precision%29) (InputAction :type Input%20Action%20Object%20Reference :default "/Game/Controls/IA_MouseInputY.IA_MouseInputY"))
  ;[1 1 1] 360 degree freedom movement rotation
  (Transformation|AddActorLocalRotation (Math|Rotator|MakeRotator 0.0 ActionValue 0.0) false false)
  ;[1 1 1] Update LineTrace for UI
  (CallFunction|UpdatedInput))

(event Input|EnhancedActionEvents|EnhancedInputActionIA_Roll
  (params (ActionValue :type Float%20%28double-precision%29) (ElapsedSeconds :type Float%20%28double-precision%29) (TriggeredSeconds :type Float%20%28double-precision%29) (InputAction :type Input%20Action%20Object%20Reference :default "/Game/Controls/IA_Roll.IA_Roll"))
  ;[1 1 1] 360 degree freedom movement rotation
  (Transformation|AddActorLocalRotation (Math|Rotator|MakeRotator ActionValue 0.0 0.0) false false)
  ;[1 1 1] Update LineTrace for UI
  (CallFunction|UpdatedInput))

(event EventBeginPlay
  ;[1 0.3613 0.3419] Add Enhanced Input System
  (bind _asplayer_controller (Utilities|Casting|CastToPlayerController (Pawn|GetController)))
  (Input|AddMappingContext (PlayerController|LocalPlayerSubsystems|GetEnhancedInputLocalPlayerSubsystem _asplayer_controller) "/Game/Controls/InputController.InputController" 0 "(bIgnoreAllPressedKeysUntilRelease=True,bForceImmediately=False,bNotifyUserSettings=False)")
  (bind _returnvalue (UserInterface|CreateWidget "/Game/UI/PlayerCharacterUI.PlayerCharacterUI_C"))
  (bind _output_get (Variables|Default|SetHUDWidget _returnvalue))
  (UserInterface|Viewport|AddtoViewport _output_get 0))

(event EventTick
  (params (DeltaSeconds :type Float%20%28single-precision%29))
  ;[1 0.8969 0.266] Debug
  (Utilities|FlowControl|Delay 0.2))

(fn ConstructionScript)