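; First-person player Character Blueprint that handles movement and horizontal mouse look through Enhanced Input.
; On BeginPlay it casts its controller to PlayerController and adds the InputController mapping context.
; Forward and side move actions feed AddMovementInput along the actor's forward and right vectors.
; Mouse X drives controller yaw, while the pitch input node is left unconnected, so vertical look is inactive.
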(event Input|EnhancedActionEvents|EnhancedInputActionIA_ForwardMove
  (params (ActionValue :type Float%20%28double-precision%29) (ElapsedSeconds :type Float%20%28double-precision%29) (TriggeredSeconds :type Float%20%28double-precision%29) (InputAction :type Input%20Action%20Object%20Reference :default "/Game/Controls/IA_ForwardMove.IA_ForwardMove"))
  (:Triggered
    (Pawn|Input|AddMovementInput (Transformation|GetActorForwardVector) ActionValue false)))

(event Input|EnhancedActionEvents|EnhancedInputActionIA_SideMove
  (params (ActionValue :type Float%20%28double-precision%29) (ElapsedSeconds :type Float%20%28double-precision%29) (TriggeredSeconds :type Float%20%28double-precision%29) (InputAction :type Input%20Action%20Object%20Reference :default "/Game/Controls/IA_SideMove.IA_SideMove"))
  (:Triggered
    (Pawn|Input|AddMovementInput (Transformation|GetActorRightVector) ActionValue false)))

(event Input|EnhancedActionEvents|EnhancedInputActionIA_MouseInput
  (params (ActionValue :type Vector%202D%20Structure) (ElapsedSeconds :type Float%20%28double-precision%29) (TriggeredSeconds :type Float%20%28double-precision%29) (InputAction :type Input%20Action%20Object%20Reference :default "/Game/Controls/IA_MouseInput.IA_MouseInput"))
  (:Triggered
    (Pawn|Input|AddControllerYawInput (.X (Math|Vector2D|BreakVector2D ActionValue)))))

(event EventBeginPlay
  (bind _asplayer_controller (Utilities|Casting|CastToPlayerController (Pawn|GetController)))
  (Input|AddMappingContext (PlayerController|LocalPlayerSubsystems|GetEnhancedInputLocalPlayerSubsystem _asplayer_controller) "/Game/Controls/InputController.InputController" 0 "(bIgnoreAllPressedKeysUntilRelease=True,bForceImmediately=False,bNotifyUserSettings=False)"))

(fn ConstructionScript)