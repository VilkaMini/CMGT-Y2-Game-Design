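; Puzzle controller that opens a door when a set of ButtonSimple actors matches a correct on/off pattern.
; Components report through Communicate, which routes by puzzle ID; only puzzle 1 is implemented, with its answer set in BeginPlay.
; When the reporting NameID belongs to that puzzle, a reusable check compares each button's Status to the answer by index, then opens the DoorList entry at the given DoorID.
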(event Custom|PuzzleCorrectCheck
  (params (ActorList :type Array%20of%20Actor%20Object%20References) (CorrectList :type Array%20of%20Booleans) (doorID :type Integer))
  ;[1 1 1] Check For Puzzle
  (bind (_array_element _array_index) (Utilities|Array|ForEachLoopwithBreak ActorList :!label _label)
    (:LoopBody
      (bind _asbutton_simple (Utilities|Casting|CastToButtonSimple _array_element))
      (if (== (Variables|/Game/Blueprints/InteractableObjects/ButtonSimple.ButtonSimple_C|GetStatus _asbutton_simple) (Utilities|Array|Get(acopy) CorrectList _array_index))
        (if (== (- (Utilities|Array|Length CorrectList) 1) _array_index)
          (for (_array_element_2 _array_index_2) (Variables|Default|GetDoorList)
            (if (== _array_index_2 doorID)
              (Default|OpenDoor _array_element_2))))
        (else
          (goto _label Break))))))

(event Custom|Puzzle1Check
  ;[1 1 1] Puzzle 1 Check and Debug
  (for _array_element (Variables|Default|GetPuzzle1List)
    (bind _asbutton_simple (Utilities|Casting|CastToButtonSimple _array_element))
    (if (Utilities|Enum|Equal(Enum) (Variables|/Game/Blueprints/InteractableObjects/ButtonSimple.ButtonSimple_C|GetNameID _asbutton_simple) (Variables|Default|GetTempNameID))
      (CallFunction|PuzzleCorrectCheck (Variables|Default|GetPuzzle1List) (Variables|Default|GetPuzzle1Correct)))))

(event EventBeginPlay
  ;[1 1 1] Correct Puzzle1 Sequence
  (Variables|Default|SetPuzzle1Correct (Utilities|Array|MakeArray true true false true false false)))

(event EventCommunicate
  (params (Status :type Boolean) (NameID :type String) (PuzzleID :type Integer))
  ;[1 1 1] Get Update from puzzle component
  (Variables|Default|SetTempStatus Status)
  (Variables|Default|SetTempNameID NameID)
  (switch int PuzzleID
    (:0
      (Development|PrintString "NotInPuzzle"))
    (:1
      (CallFunction|Puzzle1Check))))

(fn ConstructionScript)