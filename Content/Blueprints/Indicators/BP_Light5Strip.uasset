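; BP_Light5Strip is an indicator actor with a strip of five lights.
; A graph segment loops over the five light components and sets each color from the matching LightsColors entry, converted to linear color.
; That segment is not connected to any event, and BeginPlay and the construction script are empty, so the colors are never applied by this Blueprint.
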(event EventBeginPlay)

(fn ConstructionScript)