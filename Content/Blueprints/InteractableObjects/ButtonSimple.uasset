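; A simple interactable button Blueprint that toggles between pressed and released on each Interact call.
; A FlipFlop alternates between ButtonActivate and ButtonDeactivate, which play and reverse a timeline that slides ButtonCenter slightly along its local X axis.
; The Box overlap events are empty, as the proximity logic that toggles input and visibility for Player-tagged actors is disconnected.
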(event OnComponentBeginOverlap(Box)
  (params (OverlappedComponent :type Primitive%20Component%20Object%20Reference) (OtherActor :type Actor%20Object%20Reference) (OtherComp :type Primitive%20Component%20Object%20Reference) (OtherBodyIndex :type Integer) (bFromSweep :type Boolean) (SweepResult :type Hit%20Result%20Structure%20%28by%20ref%29))
  ;[1 1 1] Enable Input By Proximity
)

(event OnComponentEndOverlap(Box)
  (params (OverlappedComponent :type Primitive%20Component%20Object%20Reference) (OtherActor :type Actor%20Object%20Reference) (OtherComp :type Primitive%20Component%20Object%20Reference) (OtherBodyIndex :type Integer))
  ;[1 1 1] Enable Input By Proximity
)

(event Custom|ButtonActivate
  ;[1 1 1] Button Animation
  (bind _buttonalpha (Timeline|ButtonAnimation Play)
    (:Update
      (Transformation|SetRelativeLocation (Variables|Default|GetButtonCenter) (Math|Vector|Lerp(Vector) "0, 0, 0" "-4.000000,0.000000,0.000000" _buttonalpha) false false))))

(event Custom|ButtonDeactivate
  ;[1 1 1] Button Animation
  (bind _buttonalpha (Timeline|ButtonAnimation Reverse)
    (:Update
      (Transformation|SetRelativeLocation (Variables|Default|GetButtonCenter) (Math|Vector|Lerp(Vector) "0, 0, 0" "-4.000000,0.000000,0.000000" _buttonalpha) false false))))

(event EventInteract
  ;[1 1 1] Interaction BPI Setup
  (Utilities|FlowControl|FlipFlop
    (:A
      (CallFunction|ButtonActivate))
    (:B
      (CallFunction|ButtonDeactivate))))

(fn ConstructionScript)