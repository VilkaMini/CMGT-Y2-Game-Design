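; Interactable lamp that toggles its rect light on and off when used, with an animated button.
; The Interact event from an interaction interface flips IsOn, then plays or reverses a timeline.
; The timeline update slides the button along its local X axis and sets the light's visibility from IsOn.
; The construction script sets IsOn to true by default.
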(event Custom|LightActivate
  ;[1 1 1] Button Animation
  (bind _buttonalpha (Timeline|Timeline Play)
    (:Update
      (Transformation|SetRelativeLocation (Variables|Default|GetButton) (Math|Vector|Lerp(Vector) "0, 0, 0" "-4.000000,0.000000,0.000000" _buttonalpha) false false)
      (Rendering|SetVisibility (Variables|Default|GetRectLight) (Variables|Default|GetIsOn?) false))))

(event Custom|LightDeactivate
  ;[1 1 1] Button Animation
  (bind _buttonalpha (Timeline|Timeline Reverse)
    (:Update
      (Transformation|SetRelativeLocation (Variables|Default|GetButton) (Math|Vector|Lerp(Vector) "0, 0, 0" "-4.000000,0.000000,0.000000" _buttonalpha) false false)
      (Rendering|SetVisibility (Variables|Default|GetRectLight) (Variables|Default|GetIsOn?) false))))

(event EventInteract
  ;[1 1 1] Interaction BPI Setup
  (if (Variables|Default|GetIsOn?)
    (Variables|Default|SetIsOn? false)
    (CallFunction|LightDeactivate)
    (else
      (Variables|Default|SetIsOn? true)
      (CallFunction|LightActivate))))

(fn ConstructionScript
  (Variables|Default|SetIsOn? true))