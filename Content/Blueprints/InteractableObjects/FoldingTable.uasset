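; FoldingTable is an interactable table Blueprint that folds open and closed when the player interacts with it.
; The interaction interface event uses a FlipFlop to alternate between opening and closing.
; One timeline plays forward or in reverse, lerping the relative rotations of two hinge components so they swing to different angles together.
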(event Custom|OpenTable
  ;[1 1 1] Table Animation
  (bind _alpha (Timeline|TableAnimation Play)
    (:Update
      (Transformation|SetRelativeRotation (Variables|Default|GetHinge1) (Math|Rotator|Lerp(Rotator) "0, 0, 0" "0.000000,0.000000,90.000000" _alpha true) false false)
      (Transformation|SetRelativeRotation (Variables|Default|GetHinge2) (Math|Rotator|Lerp(Rotator) "0, 0, 0" "0.000000,0.000000,180.000010" _alpha true) false false))))

(event Custom|CloseTable
  ;[1 1 1] Table Animation
  (bind _alpha (Timeline|TableAnimation Reverse)
    (:Update
      (Transformation|SetRelativeRotation (Variables|Default|GetHinge1) (Math|Rotator|Lerp(Rotator) "0, 0, 0" "0.000000,0.000000,90.000000" _alpha true) false false)
      (Transformation|SetRelativeRotation (Variables|Default|GetHinge2) (Math|Rotator|Lerp(Rotator) "0, 0, 0" "0.000000,0.000000,180.000010" _alpha true) false false))))

(event EventInteract
  ;[1 1 1] BPI Interaction
  (Utilities|FlowControl|FlipFlop
    (:A
      (CallFunction|OpenTable))
    (:B
      (CallFunction|CloseTable))))

(fn ConstructionScript)